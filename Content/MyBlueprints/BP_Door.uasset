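; BP_Door is an interactable swinging door that shows an interact widget during sphere overlap.
; Interact is ignored while Locked or in a brief timer-reset cooldown, and toggles the door only if the third-person character's TakeKey succeeds for its KeyID.
; Toggling snaps the door between zero rotation and a yaw offset, signed by dotting the actor's forward vector with the door's right vector.
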(event OnComponentBeginOverlap(OverlapSphere)
  (params (OverlappedComponent :type Primitive%20Component%20Object%20Reference) (OtherActor :type Actor%20Object%20Reference) (OtherComp :type Primitive%20Component%20Object%20Reference) (OtherBodyIndex :type Integer) (bFromSweep :type Boolean) (SweepResult :type Hit%20Result%20Structure%20%28by%20ref%29))
  (Rendering|SetVisibility (Variables|Default|GetInteractWidget) true false))

(event OnComponentEndOverlap(OverlapSphere)
  (params (OverlappedComponent :type Primitive%20Component%20Object%20Reference) (OtherActor :type Actor%20Object%20Reference) (OtherComp :type Primitive%20Component%20Object%20Reference) (OtherBodyIndex :type Integer))
  (Rendering|SetVisibility (Variables|Default|GetInteractWidget) false false))

(event Custom|Toggle%20Door%20Open/Close
  (params (Actor :type Actor%20Object%20Reference))
  (bind _door (Variables|Default|GetDoor))
  (if (> (Math|Vector|DotProduct (Math|Vector|GetForwardVector (Math|Rotator|MakeRotator 0.0 0.0 (.yaw (Transformation|GetActorRotation Actor)))) (Math|Vector|GetRightVector (Math|Rotator|MakeRotator 0.0 0.0 (.yaw (Transformation|GetWorldRotation (Variables|Default|GetDoor)))))) 0.0)
    (Variables|Default|SetdoorRotationAmt (Math|Float|Absolute(Float) (Variables|Default|GetdoorRotationAmt)))
    (else
      (Variables|Default|SetdoorRotationAmt (* (Math|Float|Absolute(Float) (Variables|Default|GetdoorRotationAmt)) -1.0))))
  ;[1 1 1] Determining if should close or open door
  (if (Utilities|Operators|EqualEqual :A (Variables|/Script/Engine.SceneComponent|GetRelativeRotation _door))
    (Transformation|SetRelativeRotation _door (Math|Rotator|MakeRotator 0.0 0.0 (Variables|Default|GetdoorRotationAmt)) false false)
    (else
      (Transformation|SetRelativeRotation _door "0, 0, 0" false false))))

(event EventBeginPlay)

(event EventInteract
  (params (actor :type Actor%20Object%20Reference))
  (if (and (not (Variables|Default|GetbIsOnCooldown)) (not (Variables|Default|GetbLocked)))
    (Variables|Default|SetbIsOnCooldown true)
    (Utilities|Time|SetTimerbyFunctionName 0 "CooldownCallbackFunc" 0.2)
    (bind _asbp_third_person_character (Utilities|Casting|CastToBP_ThirdPersonCharacter actor))
    (bind _returnvalue (Class|HorrorGameCharacter|TakeKey _asbp_third_person_character (Variables|Default|GetKeyID)))
    (if _returnvalue
      (CallFunction|ToggleDoorOpen/Close actor))))

(event EventTick
  (params (DeltaSeconds :type Float%20%28single-precision%29)))

(fn ConstructionScript)

(fn CooldownCallbackFunc
  (Variables|Default|SetbIsOnCooldown false))