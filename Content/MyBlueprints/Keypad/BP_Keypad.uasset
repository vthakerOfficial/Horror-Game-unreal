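; BP_Keypad is an interactable keypad that generates a PIN on BeginPlay and accepts guesses through a UI widget.
; An overlap sphere shows a prompt widget to the locally controlled pawn, and Interact opens WBP_Keypad with UI-only input and a mouse cursor.
; HelperTryPin checks guesses via TryPin, swaps the mesh material to open or wrong, and permanently disables interaction on success.
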(event OnComponentBeginOverlap(OverlapSphere)
  (params (OverlappedComponent :type Primitive%20Component%20Object%20Reference) (OtherActor :type Actor%20Object%20Reference) (OtherComp :type Primitive%20Component%20Object%20Reference) (OtherBodyIndex :type Integer) (bFromSweep :type Boolean) (SweepResult :type Hit%20Result%20Structure%20%28by%20ref%29))
  (if (Variables|Default|GetbInteractable)
    (bind _aspawn (Utilities|Casting|CastToPawn OtherActor))
    (if (Pawn|IsLocallyControlled _aspawn)
      (Rendering|SetVisibility (Variables|Default|GetWidget) true false))))

(event OnComponentEndOverlap(OverlapSphere)
  (params (OverlappedComponent :type Primitive%20Component%20Object%20Reference) (OtherActor :type Actor%20Object%20Reference) (OtherComp :type Primitive%20Component%20Object%20Reference) (OtherBodyIndex :type Integer))
  (if (Variables|Default|GetbInteractable)
    (bind _aspawn (Utilities|Casting|CastToPawn OtherActor))
    (if (Pawn|IsLocallyControlled _aspawn)
      (Rendering|SetVisibility (Variables|Default|GetWidget) false false))))

(event Custom|Disable%20Interaction%20Permanently
  (Components|DestroyComponent (Variables|Default|GetOverlapSphere))
  (Components|DestroyComponent (Variables|Default|GetWidget))
  (Variables|Default|SetbInteractable false))

(event EventBeginPlay
  (Class|Keypad|CreateNewPin (Variables|Default|GetNum%20Digits)))

(event Collision|EventActorBeginOverlap
  (params (OtherActor :type Actor%20Object%20Reference)))

(event EventTick
  (params (DeltaSeconds :type Float%20%28single-precision%29)))

(event EventInteract
  (params (actor :type Actor%20Object%20Reference))
  (bind _returnvalue (Game|GetPlayerController 0))
  (if (Variables|Default|GetbInteractable)
    (bind _returnvalue_2 (UserInterface|CreateWidget "/Game/MyBlueprints/Keypad/WBP_Keypad.WBP_Keypad_C" _returnvalue self))
    (bind _output_get (Variables|Default|SetREF_WidgetKeypad _returnvalue_2))
    (UserInterface|Viewport|AddtoViewport _output_get 0)
    (Input|SetInputModeUIOnly _returnvalue _output_get "DoNotLock" true)
    (Variables|/Script/Engine.PlayerController|SetbShowMouseCursor _returnvalue true)))

(fn ConstructionScript)

(fn HelperTryPin
  (params (guess :type Integer))
  (bind _returnvalue (Class|Keypad|TryPin guess))
  (if _returnvalue
    (Rendering|Material|SetMaterial (Variables|Default|GetStaticMesh) 1 "/Game/Assets/HorrorEngineStuff/HorrorEngine/Textures/M_Digit_Open.M_Digit_Open")
    (CallFunction|DisableInteractionPermanently)
    (else
      (Rendering|Material|SetMaterial (Variables|Default|GetStaticMesh) 1 "/Game/Assets/HorrorEngineStuff/HorrorEngine/Textures/M_Digit_Wrong.M_Digit_Wrong")))
  (return _returnvalue))