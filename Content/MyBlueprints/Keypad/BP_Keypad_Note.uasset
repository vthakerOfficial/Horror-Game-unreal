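; BP_Keypad_Note is a world pickup that reveals one value of a keypad code.
; SetValueandIndex stores a value and index through the parent, prints the value on a text render and shows the note mesh.
; A sphere overlap toggles the interact widget.
; OnFound passes the value and index to the player character's keypad note widget, adding that widget if missing, then destroys the note.
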(event OnComponentBeginOverlap(Sphere)
  (params (OverlappedComponent :type Primitive%20Component%20Object%20Reference) (OtherActor :type Actor%20Object%20Reference) (OtherComp :type Primitive%20Component%20Object%20Reference) (OtherBodyIndex :type Integer) (bFromSweep :type Boolean) (SweepResult :type Hit%20Result%20Structure%20%28by%20ref%29))
  ;[1 1 1] Widget Interact Button, toggling visibility
  (Rendering|SetVisibility (Variables|Default|GetWidget) true false))

(event OnComponentEndOverlap(Sphere)
  (params (OverlappedComponent :type Primitive%20Component%20Object%20Reference) (OtherActor :type Actor%20Object%20Reference) (OtherComp :type Primitive%20Component%20Object%20Reference) (OtherBodyIndex :type Integer))
  ;[1 1 1] Widget Interact Button, toggling visibility
  (Rendering|SetVisibility (Variables|Default|GetWidget) false false))

(event Custom|On%20Found
  (bind _index (Variables|Default|Getindex))
  (bind _val (Variables|Default|Getval))
  (bind _asbp_third_person_character (Utilities|Casting|CastToBP_ThirdPersonCharacter (Game|GetPlayerCharacter 0)))
  (bind _ref_keypad_note_widget (Default|GetWidgetKeypadNote _asbp_third_person_character))
  (Utilities|IsValid _ref_keypad_note_widget
    (:Is%20Valid
      (Default|InitKeyat _ref_keypad_note_widget _index _val))
    (:Is%20Not%20Valid
      (Default|AddWidgetKeypadNote _asbp_third_person_character)
      (bind _ref_keypad_note_widget_2 (Default|GetWidgetKeypadNote _asbp_third_person_character))
      (Default|InitKeyat _ref_keypad_note_widget_2 _index _val)))
  (Actor|DestroyActor))

(event EventBeginPlay)

(event Collision|EventActorBeginOverlap
  (params (OtherActor :type Actor%20Object%20Reference)))

(event EventTick
  (params (DeltaSeconds :type Float%20%28single-precision%29)))

(event EventSetValueandIndex
  (params (newVal :type Integer) (newIndex :type Integer))
  (|CallParentFunction newVal newIndex)
  (Rendering|Components|TextRender|SetText (Variables|Default|GetTextRender) (Utilities|Text|ToText(Integer) newVal))
  (Rendering|SetVisibility (Variables|Default|GetCube) true true)
  (Rendering|SetVisibility (Variables|Default|GetWidget) false false))

(fn ConstructionScript)

(fn PickUp
  (bind _output_get (LocalVariables|SettempVar (Utilities|Struct|MakeStructItemInfo "" "" 0 self)))
  (return _output_get))