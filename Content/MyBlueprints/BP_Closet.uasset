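; Closet hiding spot that a player character can enter and exit, marking it safe while inside.
; An overlap sphere shows the interact widget only for a locally controlled pawn in range.
; Interact toggles the inside state, sets the character's safe flag, teleports it to the inside or outside reference transform and rotates the door to match.
; A short timer cooldown blocks repeated interactions.
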(event OnComponentBeginOverlap(OverlapSphere)
  (params (OverlappedComponent :type Primitive%20Component%20Object%20Reference) (OtherActor :type Actor%20Object%20Reference) (OtherComp :type Primitive%20Component%20Object%20Reference) (OtherBodyIndex :type Integer) (bFromSweep :type Boolean) (SweepResult :type Hit%20Result%20Structure%20%28by%20ref%29))
  (bind _aspawn (Utilities|Casting|CastToPawn OtherActor))
  (if (Pawn|IsLocallyControlled _aspawn)
    (Rendering|SetVisibility (Variables|Default|GetInteractWidget) true false)))

(event OnComponentEndOverlap(OverlapSphere)
  (params (OverlappedComponent :type Primitive%20Component%20Object%20Reference) (OtherActor :type Actor%20Object%20Reference) (OtherComp :type Primitive%20Component%20Object%20Reference) (OtherBodyIndex :type Integer))
  (bind _aspawn (Utilities|Casting|CastToPawn OtherActor))
  (if (Pawn|IsLocallyControlled _aspawn)
    (Rendering|SetVisibility (Variables|Default|GetInteractWidget) false false)))

(event EventBeginPlay)

(event Collision|EventActorBeginOverlap
  (params (OtherActor :type Actor%20Object%20Reference)))

(event EventTick
  (params (DeltaSeconds :type Float%20%28single-precision%29)))

(fn ConstructionScript)

(fn CooldownCallbackFunc
  (Variables|Default|SetIs%20On%20Cooldown false))

(fn Interact
  (params (actor :type Actor%20Object%20Reference))
  (bind _refout (Variables|Default|GetREFOUT))
  (bind _refin (Variables|Default|GetREFIN))
  (bind _returnvalue (Transformation|GetWorldTransform _refin))
  (bind _returnvalue_2 (Transformation|GetWorldTransform _refout))
  (if (not (Variables|Default|GetIs%20On%20Cooldown))
    (Variables|Default|SetIs%20On%20Cooldown true)
    (Utilities|Time|SetTimerbyFunctionName 0 "Cooldown Callback Func" 0.5)
    (bind _asbp_third_person_character (Utilities|Casting|CastToBP_ThirdPersonCharacter actor))
    (Class|HorrorGameCharacter|SetIsSafe _asbp_third_person_character (not (Variables|Default|GetIs%20Inside)))
    (if (Variables|Default|GetIs%20Inside)
      (Transformation|SetActorTransform actor (Math|Transform|MakeTransform (.location _returnvalue_2) (.rotation _returnvalue_2) "1.000000,1.000000,1.000000"))
      (Transformation|SetRelativeRotation (Variables|Default|GetDoor) "0.000000,20.000000,0.000000" false false)
      (Variables|Default|SetIs%20Inside false)
      (else
        (Transformation|SetActorTransform actor (Math|Transform|MakeTransform (.location _returnvalue) (.rotation _returnvalue) "1.000000,1.000000,1.000000"))
        (Transformation|SetRelativeRotation (Variables|Default|GetDoor) "0, 0, 0" false false)
        (Variables|Default|SetIs%20Inside true)))
    (return)
    (else
      (return))))