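; Base item actor that the third-person character can pick up, drop, equip and unequip, with an interact widget shown on sphere overlap.
; Pickup disables physics and collision and attaches to the character mesh socket named in ItemInfo; drop shrinks the mesh, enables physics and restores collision responses cached at BeginPlay.
; Equip and Unequip toggle visibility, while PickUp returns item info.
; OnLeftClick is a stub, and a failed ground-lock loop remains unconnected.
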(event OnComponentBeginOverlap(Sphere)
  (params (OverlappedComponent :type Primitive%20Component%20Object%20Reference) (OtherActor :type Actor%20Object%20Reference) (OtherComp :type Primitive%20Component%20Object%20Reference) (OtherBodyIndex :type Integer) (bFromSweep :type Boolean) (SweepResult :type Hit%20Result%20Structure%20%28by%20ref%29))
  ;[1 1 1] Widget Interact Button, toggling visibility
  (Rendering|SetVisibility (Variables|Default|GetWidget) true false))

(event OnComponentEndOverlap(Sphere)
  (params (OverlappedComponent :type Primitive%20Component%20Object%20Reference) (OtherActor :type Actor%20Object%20Reference) (OtherComp :type Primitive%20Component%20Object%20Reference) (OtherBodyIndex :type Integer))
  ;[1 1 1] Widget Interact Button, toggling visibility
  (Rendering|SetVisibility (Variables|Default|GetWidget) false false))

(event Custom|Unequip
  (Rendering|SetVisibility (Variables|Default|GetMesh) false false)
  (Variables|Default|SetbIsVisible false))

(event Custom|Equip
  (Rendering|SetVisibility (Variables|Default|GetMesh) true false)
  (Variables|Default|SetbIsVisible true))

(event Custom|On%20Drop
  (bind _mesh (Variables|Default|GetMesh))
  (Transformation|SetWorldScale3D _mesh (* (Variables|Default|GetREF_OrigScale) "0.500000,0.500000,0.250000"))
  (Collision|SetCollisionEnabled _mesh "QueryAndPhysics")
  (Physics|SetSimulatePhysics _mesh true)
  (Collision|SetCollisionResponsetoAllChannels (Variables|Default|GetSphere) "ECR_Overlap")
  (for (_array_element _array_index) (Variables|Default|GetALLCOLLISIONCHANNELS)
    (Collision|SetCollisionResponsetoChannel (Variables|Default|GetMesh) _array_element (Utilities|Array|Get(acopy) (Variables|Default|GetREF_CollisionChannelResponseDefaults) _array_index))))

(event Custom|On%20Pickup
  (params (Actor :type Actor%20Object%20Reference))
  (bind _mesh (Variables|Default|GetMesh))
  (Transformation|SetWorldScale3D _mesh (Variables|Default|GetREF_OrigScale))
  (Physics|SetSimulatePhysics _mesh false)
  (Collision|SetCollisionEnabled _mesh "NoCollision")
  (bind _asbp_third_person_character (Utilities|Casting|CastToBP_ThirdPersonCharacter Actor))
  (Transformation|AttachComponentToComponent (Variables|/Script/Engine.Character|GetMesh _asbp_third_person_character) (Utilities|String|StringToName (.socketName (Utilities|Struct|BreakStructItemInfo (Variables|Default|GetItemInfo)))) "SnapToTarget" "SnapToTarget" "KeepRelative" false)
  (Transformation|AddRelativeRotation (Variables|Default|GetMesh) "0.000000,90.000000,0.000000" false false)
  (Collision|SetCollisionResponsetoAllChannels (Variables|Default|GetSphere) "ECR_Ignore")
  (Rendering|SetVisibility (Variables|Default|GetWidget) false false))

(event EventBeginPlay
  (Variables|Default|SetREF_OrigScale (Transformation|GetWorldScale (Variables|Default|GetMesh)))
  (for _array_element (Variables|Default|GetALLCOLLISIONCHANNELS)
    (Utilities|Array|Add (Variables|Default|GetREF_CollisionChannelResponseDefaults) (Collision|GetCollisionResponsetoChannel (Variables|Default|GetMesh) _array_element))))

(event Collision|EventActorBeginOverlap
  (params (OtherActor :type Actor%20Object%20Reference)))

(event EventTick
  (params (DeltaSeconds :type Float%20%28single-precision%29)))

(fn ConstructionScript)

(fn OnLeftClick
  (return 0.0))

(fn PickUp
  (bind _iteminfo (Variables|Default|GetItemInfo))
  (bind (_name _socketname _icon) (Utilities|Struct|BreakStructItemInfo _iteminfo))
  (Development|PrintString "item picked")
  (return (Utilities|Struct|MakeStructItemInfo _name _socketname _icon self)))