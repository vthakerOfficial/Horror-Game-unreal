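; BP_Bat is a melee weapon pickup whose left-click attack damages and knocks back AI characters.
; OnLeftClick sphere-traces from the owner's camera along controller rotation, with debug drawing on.
; The first new "AI"-tagged hit takes damage, gets launched along control yaw with added lift, and triggers an attack montage before returning.
; OnPickup offsets the mesh, and a separate callback interpolates stored actors toward knockback targets.
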(event Custom|Apply%20Knockback%20Callback%20Func
  (params (DeltaTime :type Float%20%28double-precision%29))
  (for (_array_element _array_index) (Variables|Default|GetApplyKnockback_Actors)
    (Transformation|SetActorLocation _array_element (Math|Interpolation|VInterpTo (Transformation|GetActorLocation _array_element) (Utilities|Array|Get(acopy) (Variables|Default|GetApplyKnockback_targetLocations) _array_index) DeltaTime 0.5) false false)))

(event EventBeginPlay
  (|CallParentFunction) ; This node is disabled and will not be called.\nDrag off pins to build functionality.
)

(event Collision|EventActorBeginOverlap
  (params (OtherActor :type Actor%20Object%20Reference))
  (|CallParentFunction OtherActor) ; This node is disabled and will not be called.\nDrag off pins to build functionality.
)

(event EventTick
  (params (DeltaSeconds :type Float%20%28single-precision%29))
  (|CallParentFunction DeltaSeconds) ; This node is disabled and will not be called.\nDrag off pins to build functionality.
)

(event EventOnPickup
  (params (Actor :type Actor%20Object%20Reference))
  (|CallParentFunction Actor)
  (Transformation|AddRelativeLocation (Variables|Character|GetMesh) "-44.358903,0.795877,23.816470" false false))

(fn ConstructionScript
  (|CallParentFunction))

(fn OnLeftClick
  (|CallParentFunction)
  (bind _asbp_third_person_character (Utilities|Casting|CastToBP_ThirdPersonCharacter (Components|GetOwner)))
  (LocalVariables|SetREF_Owner _asbp_third_person_character)
  (bind _outhits (Collision|MultiSphereTraceForObjects (Transformation|GetWorldLocation (Variables|/Script/HorrorGame.HorrorGameCharacter|GetFollowCamera (LocalVariables|GetREF_Owner))) (+ (Transformation|GetWorldLocation (Variables|/Script/HorrorGame.HorrorGameCharacter|GetFollowCamera (LocalVariables|GetREF_Owner))) (* (Math|Vector|GetForwardVector (Pawn|GetDesiredRotation (Game|GetInstigatorController (LocalVariables|GetREF_Owner)))) (Variables|Default|GetAttackReach))) (Math|Vector|Distance2D(Vector) (Transformation|GetWorldLocation (Variables|/Game/Assets/ThirdPersonTemplateStuff/ThirdPerson/Blueprints/BP_ThirdPersonCharacter.BP_ThirdPersonCharacter_C|GetArrow1 (LocalVariables|GetREF_Owner))) (Transformation|GetWorldLocation (Variables|/Script/Engine.Character|GetMesh (LocalVariables|GetREF_Owner)))) (LocalVariables|GetObjectType%20for%20Sphere%20Trace) false 0 "ForDuration" true "(R=1.000000,G=0.000000,B=0.000000,A=1.000000)" "(R=0.000000,G=1.000000,B=0.000000,A=1.000000)" 2.0))
  (for _array_element _outhits
    (if (and (Actor|ActorHasTag (.HitActor (Collision|BreakHitResult _array_element)) "AI") (not (Utilities|Array|ContainsItem (LocalVariables|GetalreadyHitActors) (.HitActor (Collision|BreakHitResult _array_element)))))
      (Utilities|Array|Add (LocalVariables|GetalreadyHitActors) (.HitActor (Collision|BreakHitResult _array_element)))
      (Development|PrintString "found a monster")
      (Game|Damage|ApplyDamage (.HitActor (Collision|BreakHitResult _array_element)) (Variables|Default|GetDamage%20Amount) (Pawn|GetController (LocalVariables|GetREF_Owner)) self)
      (bind _asbp_ai (Utilities|Casting|CastToBP_AI (.HitActor (Collision|BreakHitResult _array_element))))
      (Character|LaunchCharacter _asbp_ai (Math|Vector|MakeVector (.x (* (Math|Vector|GetForwardVector (Math|Rotator|MakeRotator 0.0 0.0 (.yaw (Pawn|GetControlRotation (Pawn|GetController (LocalVariables|GetREF_Owner)) :!class /Script/Engine.Controller)))) (Variables|Default|GetLaunch%20Force))) (.y (* (Math|Vector|GetForwardVector (Math|Rotator|MakeRotator 0.0 0.0 (.yaw (Pawn|GetControlRotation (Pawn|GetController (LocalVariables|GetREF_Owner)) :!class /Script/Engine.Controller)))) (Variables|Default|GetLaunch%20Force))) (+ (.z (* (Math|Vector|GetForwardVector (Math|Rotator|MakeRotator 0.0 0.0 (.yaw (Pawn|GetControlRotation (Pawn|GetController (LocalVariables|GetREF_Owner)) :!class /Script/Engine.Controller)))) (Variables|Default|GetLaunch%20Force))) 3.5e+02)) true true)
      (Default|OnKnockback _asbp_ai)
      (bind _returnvalue (Animation|PlayAnimMontage (LocalVariables|GetREF_Owner) "/Game/MyAI/Animation/NewMixamo/Zombie_Attack_Anim_mixamo_com_Montage.Zombie_Attack_Anim_mixamo_com_Montage" 1.0 "None"))
      (return _returnvalue)))
  (Utilities|Array|Clear (LocalVariables|GetalreadyHitActors)))