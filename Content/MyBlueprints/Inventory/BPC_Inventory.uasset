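; Inventory component that stores picked-up items and tracks which one the player has equipped.
; AddItem sends nameless items to keypad notes as found; others are stored, owned by the player and auto-equipped through BP_BaseItem calls.
; Tab toggles the inventory widget with cursor and input mode, rebuilding it on additions while open.
; Left click is forwarded to the equipped item, and dropping notifies the item before removing it.
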(event Custom|Open%20Inventory
  (bind _returnvalue (Game|GetPlayerController 0))
  ;[1 1 1] Inventory Open/Close/Update
  (bind _returnvalue_2 (UserInterface|CreateWidget "/Game/MyBlueprints/Inventory/WBP_Inventory.WBP_Inventory_C" _returnvalue))
  (bind _output_get (Variables|Default|SetREF_Inventory _returnvalue_2))
  (UserInterface|Viewport|AddtoViewport _output_get 0)
  (Input|SetInputModeGameandUI _returnvalue 0 "DoNotLock" true false)
  (Variables|/Script/Engine.PlayerController|SetbShowMouseCursor _returnvalue true))

(event Custom|Close%20Inventory
  (bind _returnvalue (Game|GetPlayerController 0))
  ;[1 1 1] Inventory Open/Close/Update
  (Widget|RemovefromParent (Variables|Default|GetREF_Inventory))
  (Variables|Default|SetREF_Inventory 0)
  (Variables|/Script/Engine.PlayerController|SetbShowMouseCursor _returnvalue false)
  (Input|SetInputModeGameOnly _returnvalue false))

(event Custom|Update%20Inventory
  ;[1 1 1] Inventory Open/Close/Update
  (Utilities|IsValid (Variables|Default|GetREF_Inventory)
    (:Is%20Valid
      (Widget|RemovefromParent (Variables|Default|GetREF_Inventory))
      (bind _returnvalue (UserInterface|CreateWidget "/Game/MyBlueprints/Inventory/WBP_Inventory.WBP_Inventory_C"))
      (bind _output_get (Variables|Default|SetREF_Inventory _returnvalue))
      (UserInterface|Viewport|AddtoViewport _output_get 0))))

(event Custom|Add%20Item
  (params (NewItem :type Struct%20Item%20Info%20Structure%20%28by%20ref%29))
  (bind (_name _socketname _icon _itemref) (Utilities|Struct|BreakStructItemInfo NewItem))
  (bind _inventory (Variables|Default|GetInventory))
  (if (Utilities|Enum|Equal(Enum) _name "")
    (bind _asbp_keypad_note (Utilities|Casting|CastToBP_Keypad_Note _itemref))
    (Default|OnFound _asbp_keypad_note)
    (else
      (Utilities|Array|Add _inventory NewItem)
      (CallFunction|UpdateInventory)
      (bind _asbp_base_item (Utilities|Casting|CastToBP_BaseItem (.itemRef (Utilities|Struct|BreakStructItemInfo NewItem))))
      (Actor|SetOwner _asbp_base_item (Game|GetPlayerCharacter 0))
      (Default|OnPickup _asbp_base_item (Game|GetPlayerCharacter 0))
      (CallFunction|EquipItem (- (Utilities|Array|Length _inventory) 1)))))

(event Custom|Drop%20Item
  (params (Index :type Integer))
  (bind _asbp_base_item (Utilities|Casting|CastToBP_BaseItem (.itemref (Utilities|Array|Get(acopy) (Variables|Default|GetInventory) Index))))
  (Default|OnDrop _asbp_base_item)
  (Utilities|Array|RemoveIndex (Variables|Default|GetInventory) Index)
  (Development|PrintString "Hello"))

(event Custom|Equip%20Item
  (params (New%20Equipped%20Index :type Integer))
  (bind _newparam (CallFunction|GetEquippedItem))
  (Utilities|IsValid _newparam
    (:Is%20Valid
      (Default|Unequip _newparam))
    (:Is%20Not%20Valid
      _))
  (Variables|Default|SetEquipped%20Index New%20Equipped%20Index)
  (bind _newparam_2 (CallFunction|GetEquippedItem))
  (Utilities|IsValid _newparam_2
    (:Is%20Valid
      (Default|Equip _newparam_2))))

(event Input|KeyboardEvents|Tab
  (params (Key :type Key%20Structure :default "None"))
  ;[1 1 1] Inventory Open/Close/Update
  (:Pressed
    (Utilities|FlowControl|FlipFlop
      (:A
        (CallFunction|OpenInventory))
      (:B
        (CallFunction|CloseInventory)))))

(event Input|MouseEvents|LeftMouseButton
  (params (Key :type Key%20Structure :default "None"))
  (:Pressed
    (bind _newparam (CallFunction|GetEquippedItem))
    (Utilities|IsValid _newparam
      (:Is%20Valid
        (Default|OnLeftClick _newparam)))))

(fn GetEquippedItem
  (bind _inventory (Variables|Default|GetInventory))
  (bind _equipped_index (Variables|Default|GetEquipped%20Index))
  (if (Utilities|Array|IsValidIndex _inventory _equipped_index)
    (bind _asbp_base_item (Utilities|Casting|CastToBP_BaseItem (.itemRef (Utilities|Struct|BreakStructItemInfo (Utilities|Array|Get(acopy) _inventory _equipped_index)))))
    (return _asbp_base_item)))