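; BP_Closet is an interactable closet that an actor can step into and out of.
; Interact toggles IsInside, teleporting the actor to the REFIN or REFOUT reference transform and snapping the Door's rotation to match.
; A Sphere overlap shows and hides the Widget, while the Trigger overlap does nothing.
; Interact also sets a timer by function name; CooldownCallbackFunc sets IsOnCooldown, but nothing here checks that flag.
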(event OnComponentBeginOverlap(Trigger)
  (params (OverlappedComponent :type Primitive%20Component%20Object%20Reference) (OtherActor :type Actor%20Object%20Reference) (OtherComp :type Primitive%20Component%20Object%20Reference) (OtherBodyIndex :type Integer) (bFromSweep :type Boolean) (SweepResult :type Hit%20Result%20Structure%20%28by%20ref%29)))

(event OnComponentBeginOverlap(Sphere)
  (params (OverlappedComponent :type Primitive%20Component%20Object%20Reference) (OtherActor :type Actor%20Object%20Reference) (OtherComp :type Primitive%20Component%20Object%20Reference) (OtherBodyIndex :type Integer) (bFromSweep :type Boolean) (SweepResult :type Hit%20Result%20Structure%20%28by%20ref%29))
  (Rendering|SetVisibility (Variables|Default|GetWidget) true false))

(event OnComponentEndOverlap(Sphere)
  (params (OverlappedComponent :type Primitive%20Component%20Object%20Reference) (OtherActor :type Actor%20Object%20Reference) (OtherComp :type Primitive%20Component%20Object%20Reference) (OtherBodyIndex :type Integer))
  (Rendering|SetVisibility (Variables|Default|GetWidget) false false))

(event EventBeginPlay)

(event Collision|EventActorBeginOverlap
  (params (OtherActor :type Actor%20Object%20Reference)))

(event EventTick
  (params (DeltaSeconds :type Float%20%28single-precision%29)))

(event EventInteract
  (params (actor :type Actor%20Object%20Reference))
  (bind _refout (Variables|Default|GetREFOUT))
  (bind _refin (Variables|Default|GetREFIN))
  (bind _returnvalue (Transformation|GetWorldTransform _refin))
  (bind _returnvalue_2 (Transformation|GetWorldTransform _refout))
  (Utilities|Time|SetTimerbyFunctionName 0 (Variables|Default|GetFunction%20Name) 0.0)
  (if (Variables|Default|GetIs%20Inside)
    (Transformation|SetActorTransform actor (Math|Transform|MakeTransform (.location _returnvalue_2) (.rotation _returnvalue_2) "1.000000,1.000000,1.000000"))
    (Transformation|SetRelativeRotation (Variables|Default|GetDoor) "0.000000,180.000000,0.000000" false false)
    (Variables|Default|SetIs%20Inside false)
    (else
      (Transformation|SetActorTransform actor (Math|Transform|MakeTransform (.location _returnvalue) (.rotation _returnvalue) "1.000000,1.000000,1.000000"))
      (Transformation|SetRelativeRotation (Variables|Default|GetDoor) "0, 0, 0" false false)
      (Variables|Default|SetIs%20Inside true))))

(fn ConstructionScript)

(fn CooldownCallbackFunc
  (Variables|Default|SetIs%20On%20Cooldown true))