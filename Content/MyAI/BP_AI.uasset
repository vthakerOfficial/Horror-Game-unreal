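; BP_AI is an AI-controlled enemy character that suspends its behavior tree while it is knocked back.
; On knockback it sets a flag, stops the brain component's logic and starts a three-second retriggerable delay, which repeated hits extend.
; Landing, or the delay expiring first, clears the flag and restarts BT_EnemyAI.
; An empty end-stun callback and its timer are left unconnected.
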(event Custom|On%20Knockback
  (if (Variables|Default|GetbHasTakenKB)
    _
    (else
      (bind _asaicontroller (Utilities|Casting|CastToAIController (Pawn|GetController)))
      (AI|Logic|StopLogic (Variables|/Script/AIModule.AIController|GetBrainComponent _asaicontroller) "Has Taken KB")
      (Variables|Default|SetbHasTakenKB true)))
  (Utilities|FlowControl|RetriggerableDelay 3.0)
  (if (Variables|Default|GetbHasTakenKB)
    (Variables|Default|SetbHasTakenKB false)
    (AI|RunBehaviorTree (AI|GetAIController 0) "/Game/MyAI/BT_EnemyAI.BT_EnemyAI")))

(event Custom|End%20Stun%20Callback%20Func)

(event EventBeginPlay)

(event Collision|EventActorBeginOverlap
  (params (OtherActor :type Actor%20Object%20Reference)))

(event EventTick
  (params (DeltaSeconds :type Float%20%28single-precision%29)))

(event EventOnLanded
  (params (Hit :type Hit%20Result%20Structure%20%28by%20ref%29))
  (|CallParentFunction Hit)
  (if (Variables|Default|GetbHasTakenKB)
    (Variables|Default|SetbHasTakenKB false)
    (bind _asaicontroller (Utilities|Casting|CastToAIController (Pawn|GetController)))
    (AI|RunBehaviorTree _asaicontroller "/Game/MyAI/BT_EnemyAI.BT_EnemyAI")))

(fn ConstructionScript)